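; Tile-based world map manager that grows the map around every BP_PLAYER and persists it in the "worldMap" save slot.
; A looping StretchMap timer converts player positions to grid cells and writes missing cells within DiameterStretchingMap to MAP_SAVED.
; A looping LoadMap timer reloads that save, creating it if needed, and ReceiveMap spawns or updates BP_TILE actors.
; The save game is the data channel between stretching and spawning, polled asynchronously.
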(event `self.ReceiveBeginPlay`
  (`KismetSystemLibrary.K2_SetTimer` null "LoadMap" 0.1 true)
  (`KismetSystemLibrary.K2_SetTimer` null "StretchMap" 0.1 true 1.0))

(event `StretchMap`
  (set `self.TilesSize` (* (`.BoxExtent` (`self.GetActorBounds` (`BlueprintMapLibrary.Map_Find` (`self.tilesArray`)) false false)) 2.0))
  (bind _outactors (`GameplayStatics.GetAllActorsOfClass` "/Game/PROJECT/PLAYER/BP_PLAYER.BP_PLAYER_C"))
  (for _array_element _outactors
    (bind _newparam1 (`self.CalculateAroundTiles` (`KismetMathLibrary.MakeVector2D` (`KismetMathLibrary.Conv_IntToDouble` (`KismetMathLibrary.FFloor` (.x (/ (`self.K2_GetActorLocation` _array_element) (`self.TilesSize`))))) (`KismetMathLibrary.Conv_IntToDouble` (`KismetMathLibrary.FFloor` (.y (/ (`self.K2_GetActorLocation` _array_element) (`self.TilesSize`))))))))
    (for _array_element_2 _newparam1
      (if (not (`.ReturnValue` (`BlueprintMapLibrary.Map_Find` (`self.tilesArray`) _array_element_2)))
        (`KismetSystemLibrary.PrintString` (`KismetStringLibrary.Conv_Vector2dToString` _array_element_2))
        (bind _savegame (`AsyncActionHandleSaveGame.AsyncLoadGameFromSlot` "worldMap")
          (:`then`
            (bind _asmap_saved (cast `/Game/PROJECT/MAP/MAP_SAVED` _savegame))
            (`BlueprintMapLibrary.Map_Add` (`/Game/PROJECT/MAP/MAP_SAVED.TILES_ARRAY` _asmap_saved) _array_element_2 "NewEnumerator0")
            (`AsyncActionHandleSaveGame.AsyncSaveGameToSlot` _savegame "worldMap")))))))

(event `self.ReceiveTick`
  (params (DeltaSeconds :type "Float (single-precision)")))

(event `ReceiveMap`
  (params (`TILES ARRAY` :type "Map of Vector2D Structure to /Game/PROJECT/MAP/ENU_presettedTiles Enum"))
  (bind _keys (`BlueprintMapLibrary.Map_Keys` `TILES ARRAY`))
  (for _array_element _keys
    (bind (_value _returnvalue) (`BlueprintMapLibrary.Map_Find` (`self.tilesArray`) _array_element))
    (if _returnvalue
      (bind _value_2 (`BlueprintMapLibrary.Map_Find` `TILES ARRAY` _array_element))
      (`/Game/PROJECT/TILE/BP_TILE.SetValue` _value _value_2)
      (else
        (bind _returnvalue_2 (`|SpawnActorFromClass` "/Game/PROJECT/TILE/BP_TILE.BP_TILE_C" (`KismetMathLibrary.MakeTransform` (0.0 0.0 0.0) (struct :`Roll` 90.0)) "AlwaysSpawn" "MultiplyWithRoot" self _value_2 null))
        (`BlueprintMapLibrary.Map_Add` (`self.tilesArray`) _array_element _returnvalue_2)
        (bind (_x _y) (`KismetMathLibrary.BreakVector2D` _array_element))
        (`self.K2_SetActorLocation` _returnvalue_2 (`KismetMathLibrary.MakeVector` (* _x (.x (`.BoxExtent` (`self.GetActorBounds` _returnvalue_2 false false))) 2.0) (* _y (.y (`.BoxExtent` (`self.GetActorBounds` _returnvalue_2 false false))) 2.0)) false false)))))

(event `LoadMap`
  (bind _savegame (`AsyncActionHandleSaveGame.AsyncLoadGameFromSlot` "worldMap")
    (:`then`
      (bind _asmap_saved (cast `/Game/PROJECT/MAP/MAP_SAVED` _savegame)
        (:`then`
          (`self.ReceiveMap` (`/Game/PROJECT/MAP/MAP_SAVED.TILES_ARRAY` _asmap_saved)))
        (:`CastFailed`
          (bind _returnvalue (`GameplayStatics.CreateSaveGameObject` "/Game/PROJECT/MAP/MAP_SAVED.MAP_SAVED_C"))
          (`AsyncActionHandleSaveGame.AsyncSaveGameToSlot` _returnvalue "worldMap"
            (:`then`
              (`self.ReceiveMap` (`/Game/PROJECT/MAP/MAP_SAVED.TILES_ARRAY` _returnvalue)))))))))

(fn `CalculateAroundTiles`
  (params (NewParam :type "Vector2D Structure"))
  (returns (NewParam1 :type "Array of Vector2D Structure"))
  (locals (tmpAroundTiles :type "Array of Vector2D Structure"))
  (bind _diameterstretchingmap (`self.diameterStretchingMap`))
  (bind _diameterstretchingmap_2 (`self.diameterStretchingMap`))
  (`KismetArrayLibrary.Array_Add` (`local.tmpAroundTiles`) NewParam)
  (for _index (range (* _diameterstretchingmap_2 -1) (+ _diameterstretchingmap_2 1))
    (for _index_2 (range (* _diameterstretchingmap -1) (+ _diameterstretchingmap 1))
      (`KismetArrayLibrary.Array_Add` (`local.tmpAroundTiles`) (+ (`local.NewParam`) (`KismetMathLibrary.MakeVector2D` (`KismetMathLibrary.Conv_IntToDouble` _index_2) (`KismetMathLibrary.Conv_IntToDouble` _index))))))
  (return (`local.tmpAroundTiles`)))

(fn `UserConstructionScript`)